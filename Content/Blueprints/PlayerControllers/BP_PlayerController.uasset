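; BP_PlayerController is the player controller that owns the HUD and keeps its fuel display current.
; On BeginPlay it creates WBP_HUD, adds it to the viewport and caches the player pawn as a BP_Ship.
; Every Tick it polls the ship's fuel percent and pushes it to the HUD, printing an error if either reference is invalid.
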(event EventBeginPlay
  (bind _returnvalue (UserInterface|CreateWidget "/Game/UI/WBP_HUD.WBP_HUD_C"))
  (bind _output_get (Variables|Default|SetHUDref _returnvalue))
  (UserInterface|Viewport|AddtoViewport _output_get 0)
  (bind _asbp_ship (Utilities|Casting|CastToBP_Ship (Game|Player|GetPlayerPawn 0))
    (:then
      (Variables|Default|SetShipRef _asbp_ship))
    (:CastFailed
      (Development|PrintString "Error: Failed to cast Player Pawn to BP Ship!"))))

(event EventTick
  (params (DeltaSeconds :type Float%20%28single-precision%29))
  (bind _hudref (Variables|Default|GetHUDref))
  (bind _shipref (Variables|Default|GetShipRef))
  (Utilities|IsValid _hudref
    (:Is%20Valid
      (Utilities|IsValid _shipref
        (:Is%20Valid
          (bind _returnvalue (Class|Ship|GetFuelPercent _shipref))
          (Default|UpdateFuel _hudref _returnvalue))
        (:Is%20Not%20Valid
          (Development|PrintString "Error: ShipRef is not valid!"))))
    (:Is%20Not%20Valid
      (Development|PrintString "Error: HUDref is not valid!"))))

(fn ConstructionScript)