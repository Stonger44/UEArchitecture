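; Player controller for the main menu that shows the menu UI over a dedicated camera view.
; On BeginPlay it creates, caches and adds WBP_MainMenu to the viewport, then looks up the CameraActor tagged MainMenuCamera.
; If exactly one exists, it becomes the view target and input switches to Game and UI with the New Game button focused; otherwise an error is printed.
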(event EventBeginPlay
  ;[0.15 0.15 0.15 0.5] Create and Cache WBP_MainMenu
  (bind _returnvalue (UserInterface|CreateWidget "/Game/UI/WBP_MainMenu.WBP_MainMenu_C"))
  (bind _output_get (Variables|Default|SetWBP_MainMenu _returnvalue))
  (UserInterface|Viewport|AddtoViewport _output_get 0)
  ;[0.15 0.15 0.15 0.5] Main Menu Camera
  (bind _outactors (Actor|GetAllActorsOfClasswithTag "/Script/Engine.CameraActor" "MainMenuCamera"))
  (if (== (Utilities|Array|Length _outactors) 1)
    (bind _output_get_2 (Variables|Default|SetMainMenuCamera (Utilities|Array|Get(acopy) _outactors)))
    (Game|Player|SetViewTargetwithBlend _output_get_2 0.0 "VTBlend_Linear" 0.0 false)
    ;[0.15 0.15 0.15 0.5] Input Mode Game and UI
    (Input|SetInputModeGameandUI self (Variables|/Game/UI/WBP_MainMenu.WBP_MainMenu_C|GetNewGameButton (Variables|Default|GetWBP_MainMenu)) "DoNotLock" true false)
    (else
      (Development|PrintString "Error finding Main Menu Camera!"))))

(event EventTick
  (params (DeltaSeconds :type Float%20%28single-precision%29)))

(fn ConstructionScript)