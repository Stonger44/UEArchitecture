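; Player controller for the lander game that owns the HUD, pause, level title and end-play widgets and switches input modes between them.
; BeginPlay shows the pause menu as a one-time intro on the starting level, tracked in the game instance, otherwise the level title.
; Tick feeds ship fuel to the HUD, pause toggling is blocked after landing, crashing or exploding, and level changes forward to the game mode.
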(event Custom|TriggerLevelTitle
  (UserInterface|Viewport|AddtoViewport (Variables|Default|GetWBP_LevelTitle) 0)
  (Variables|Default|SetbHasShownLevelTitle true))

(event Input|EnhancedActionEvents|EnhancedInputActionIA_TogglePauseMenu
  (params (ActionValue :type Boolean) (ElapsedSeconds :type Float%20%28double-precision%29) (TriggeredSeconds :type Float%20%28double-precision%29) (InputAction :type Input%20Action%20Object%20Reference :default "/Game/Blueprints/Pawns/Input/Actions/IA_TogglePauseMenu.IA_TogglePauseMenu"))
  (bind _ship (Variables|Default|GetShip))
  (bind _shipstatus (Variables|/Script/UEArchitecture.Ship|GetShipStatus _ship))
  (if (not (Math|Boolean|ORBoolean (Utilities|Enum|Equal(Enum) _shipstatus "Landed") (Utilities|Enum|Equal(Enum) _shipstatus "Crashed") (Utilities|Enum|Equal(Enum) _shipstatus "Exploded")))
    (if (Variables|Default|GetbIsGamePaused)
      (CallFunction|HidePauseMenu)
      (else
        (CallFunction|ShowPauseMenu)))))

(event EventBeginPlay
  (bind _asbp_lander_game_mode (Utilities|Casting|CastToBP_LanderGameMode (Game|GetGameMode))
    (:then
      (Variables|Default|SetLanderGameMode _asbp_lander_game_mode)
      (bind _returnvalue (UserInterface|CreateWidget "/Game/UI/WBP_HUD.WBP_HUD_C" self))
      (bind _output_get (Variables|Default|SetWBP_HUD _returnvalue))
      (UserInterface|Viewport|AddtoViewport _output_get 0)
      (bind _asbp_ship (Utilities|Casting|CastToBP_Ship (Game|Player|GetPlayerPawn 0))
        (:then
          (Variables|Default|SetShip _asbp_ship)
          (bind _returnvalue_2 (UserInterface|CreateWidget "/Game/UI/WBP_PauseMenu.WBP_PauseMenu_C" self))
          (Variables|Default|SetWBP_PauseMenu _returnvalue_2)
          (bind _returnvalue_3 (UserInterface|CreateWidget "/Game/UI/WBP_LevelTitle.WBP_LevelTitle_C" self (Class|LanderGameMode|GetLevelTitle (Variables|Default|GetLanderGameMode))))
          (Variables|Default|SetWBP_LevelTitle _returnvalue_3)
          (bind _returnvalue_4 (Game|GetCurrentLevelName true))
          (if (Utilities|Enum|Equal(Enum) _returnvalue_4 (Variables|Default|GetStartingLevelName))
            (bind _asbp_lander_game_instance (Utilities|Casting|CastToBP_LanderGameInstance (Game|GetGameInstance))
              (:then
                (if (Variables|/Game/Blueprints/GameInstances/BP_LanderGameInstance.BP_LanderGameInstance_C|GetbHasShownIntroMenu _asbp_lander_game_instance)
                  (CallFunction|HidePauseMenu)
                  (else
                    ;[0.15 0.15 0.15 0.5] Let Camera finish first
                    (Utilities|FlowControl|Delay 0.1)
                    (CallFunction|ShowPauseMenu)
                    (Variables|/Game/Blueprints/GameInstances/BP_LanderGameInstance.BP_LanderGameInstance_C|SetbHasShownIntroMenu _asbp_lander_game_instance true))))
              (:CastFailed
                (Development|PrintString "Failed to cast to BP_LanderGameInstance")))
            (else
              (CallFunction|EnableInputModeGame)
              (CallFunction|TriggerLevelTitle))))
        (:CastFailed
          (Development|PrintString "Error: Failed to cast Player Pawn to BP Ship!"))))
    (:CastFailed
      (Development|PrintString "Failed to Cast to BP_LanderGameMode"))))

(event EventTick
  (params (DeltaSeconds :type Float%20%28single-precision%29))
  (bind _wbp_hud (Variables|Default|GetWBP_HUD))
  (bind _ship (Variables|Default|GetShip))
  (Utilities|IsValid _wbp_hud
    (:Is%20Valid
      (Utilities|IsValid _ship
        (:Is%20Valid
          (Default|UpdateFuel _wbp_hud (Class|Ship|GetFuelPercent _ship)))
        (:Is%20Not%20Valid
          (Development|PrintString "Error: Ship is not valid!"))))
    (:Is%20Not%20Valid
      (Development|PrintString "Error: HUD is not valid!"))))

(event EventShowEndPlayMenu
  (params (EndPlayState :type EEndPlayState%20Enum :default "GameOver"))
  (bind _returnvalue (UserInterface|CreateWidget "/Game/UI/WBP_EndPlayMenu.WBP_EndPlayMenu_C" self EndPlayState))
  (UserInterface|Viewport|AddtoViewport _returnvalue 0)
  (CallFunction|EnableInputModeUI))

(fn ConstructionScript)

(fn EnableInputModeUI
  (Input|SetInputModeUIOnly self 0 "DoNotLock" false)
  (Variables|Default|SetbShowMouseCursor true))

(fn EnableInputModeGame
  (Input|SetInputModeGameOnly self false)
  (Variables|Default|SetbShowMouseCursor false))

(fn EnableInputModeGameandUI
  (params (WidgetToFocus :type Widget%20Object%20Reference))
  (Input|SetInputModeGameandUI self 0 "DoNotLock" true false)
  (Variables|Default|SetbShowMouseCursor true))

(fn ShowPauseMenu
  (bind _wbp_pausemenu (Variables|Default|GetWBP_PauseMenu))
  (Game|SetGamePaused true)
  (UserInterface|Viewport|AddtoViewport _wbp_pausemenu 0)
  (Input|SetInputModeGameandUI self 0 "DoNotLock" true false)
  (Default|ShowPauseMenu _wbp_pausemenu)
  (Variables|Default|SetbIsGamePaused true))

(fn HidePauseMenu
  (Default|HidePauseMenu (Variables|Default|GetWBP_PauseMenu))
  (Game|SetGamePaused false)
  (CallFunction|EnableInputModeGame)
  (Variables|Default|SetbIsGamePaused false)
  (if (not (Variables|Default|GetbHasShownLevelTitle))
    (CallFunction|TriggerLevelTitle)))

(fn RestartCurrentLevel
  (bind _landergamemode (Variables|Default|GetLanderGameMode))
  (Utilities|IsValid _landergamemode
    (:Is%20Valid
      (Class|LanderGameMode|RestartCurrentLevel _landergamemode))))

(fn LoadNextLevel
  (bind _landergamemode (Variables|Default|GetLanderGameMode))
  (Utilities|IsValid _landergamemode
    (:Is%20Valid
      (Class|LanderGameMode|LoadNextLevel _landergamemode))))

(fn LoadMainMenu
  (bind _landergamemode (Variables|Default|GetLanderGameMode))
  (Utilities|IsValid _landergamemode
    (:Is%20Valid
      (Class|LanderGameMode|LoadMainMenu _landergamemode))))

(fn QuitGame
  (Game|QuitGame self "Quit" false))